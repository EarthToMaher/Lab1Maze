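; BouncePad is an actor that teleports whatever hits it to the dungeon generator's first arrow location and triggers more dungeon spawning.
; On BeginPlay it finds the Dungeon_Generator in the level and caches it.
; Its Hit event moves the other actor to FirstArrowLoc without sweeping, then calls SpawnMore on the generator.
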(event `self.ReceiveActorBeginOverlap`
  (params (OtherActor :type "Actor Object Reference")))

(event `self.ReceiveBeginPlay`
  (bind _returnvalue (`GameplayStatics.GetActorOfClass` "/Game/Blueprints/ProceduralDungeon/Dungeon_Generator.Dungeon_Generator_C"))
  (set `self.DungeonGenerator` _returnvalue))

(event `self.ReceiveHit`
  (params (MyComp :type "PrimitiveComponent Object Reference") (Other :type "Actor Object Reference") (OtherComp :type "PrimitiveComponent Object Reference") (bSelfMoved :type Boolean) (HitLocation :type "Vector Structure") (HitNormal :type "Vector Structure") (NormalImpulse :type "Vector Structure") (Hit :type "HitResult Structure (by ref)"))
  (bind _output_get (set `self.Other` Other))
  (`self.K2_SetActorLocation` (`self.Other`) (`/Game/Blueprints/ProceduralDungeon/Dungeon_Generator.firstArrowLoc` (`self.DungeonGenerator`)) false false)
  (`/Game/Blueprints/ProceduralDungeon/Dungeon_Generator.SpawnMore` (`self.DungeonGenerator`)))

(fn `UserConstructionScript`)