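; Procedural dungeon generator that chains random rooms from a start room at BeginPlay, again a second later, and via SpawnMore.
; Rooms attach at random open exits; after a zero delay, overlap boxes are checked and colliding rooms are destroyed and retried.
; When the room count runs out, it spawns a bounce pad, sets the next start point above it, walls remaining exits and resets the count.
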(event `self.ReceiveBeginPlay`
  (`self.Spawn Start Room`)
  (`self.Spawn Next Room`)
  (`KismetSystemLibrary.Delay` 1.0)
  (`self.Spawn Start Room`)
  (`self.Spawn Next Room`))

(event `Spawn Start Room`
  (bind _tp_location (`KismetMathLibrary.BreakTransform` (`self.tp`)))
  ;[0.02053 0.3073 0.0393] Spawn Start Room
  (`KismetArrayLibrary.Array_Clear` (`self.exits List`))
  (bind _returnvalue (`|SpawnActorFromClass` "/Game/Blueprints/ProceduralDungeon/Dungeon_Room_1.Dungeon_Room_1_C" (`KismetMathLibrary.MakeTransform` _tp_location) "AlwaysSpawn" "MultiplyWithRoot" null null))
  (`KismetArrayLibrary.Array_Append` (`self.exits List`) (`SceneComponent.GetChildrenComponents` (`/Game/Blueprints/ProceduralDungeon/Master_Room.exits Folder` _returnvalue) false))
  (set `self.firstArrowLoc` (`SceneComponent.K2_GetComponentLocation` (`/Game/Blueprints/ProceduralDungeon/Master_Room.Arrow` _returnvalue))))

(event `Spawn Next Room`
  ;[0.0472 0.3316 0.13] Spawn Next Room
  (set `self.SelectedexitPoint` (`KismetArrayLibrary.Array_Random` (`self.exits List`)))
  (bind _returnvalue (`|SpawnActorFromClass` (`KismetArrayLibrary.Array_Random` (`self.RoomList`)) (`SceneComponent.K2_GetComponentToWorld` (`self.SelectedexitPoint`)) "Undefined" "MultiplyWithRoot" null null))
  (bind _asmaster_room (cast `/Game/Blueprints/ProceduralDungeon/Master_Room` _returnvalue))
  (set `self.LatestRoom` _asmaster_room)
  (`KismetSystemLibrary.Delay` 0.0)
  (`self.Check for Overlap`))

(event `Add Overlaping Rooms to List`
  ;[0.05318 0.2691 0.062] Check for Overlapping Rooms
  (for _array_element (`SceneComponent.GetChildrenComponents` (`/Game/Blueprints/ProceduralDungeon/Master_Room.Overlap Folder` (`self.LatestRoom`)) false)
    (bind _asbox_collision (cast `BoxComponent` _array_element))
    (`KismetArrayLibrary.Array_Append` (`self.OverlappedList`) (`PrimitiveComponent.GetOverlappingComponents` _asbox_collision))))

(event `Check for Overlap`
  (bind (_returnvalue_location _returnvalue_rotation) (`KismetMathLibrary.BreakTransform` (`SceneComponent.K2_GetComponentToWorld` (`/Game/Blueprints/ProceduralDungeon/Master_Room.Arrow` (`self.LatestRoom`)))))
  ;[0.09565 0.349 0.1003] Delete If Overlap
  (`self.Add Overlaping Rooms to List`)
  (if (`KismetArrayLibrary.Array_IsEmpty` (`self.OverlappedList`))
    (`KismetArrayLibrary.Array_RemoveItem` (`self.exits List`) (`self.SelectedexitPoint`))
    (`KismetArrayLibrary.Array_Clear` (`self.OverlappedList`))
    (`/Engine/EditorBlueprintResources/StandardMacros.DecrementInt` (`self.RoomAmount`)
      (:`  `
        (`KismetArrayLibrary.Array_Append` (`self.exits List`) (`SceneComponent.GetChildrenComponents` (`/Game/Blueprints/ProceduralDungeon/Master_Room.exits Folder` (`self.LatestRoom`)) false))
        (if (> (`self.RoomAmount`) 0)
          (`self.Spawn Next Room`)
          (else
            (bind _returnvalue (`|SpawnActorFromClass` "/Game/Blueprints/BouncePad.BouncePad_C" (`KismetMathLibrary.MakeTransform` _returnvalue_location _returnvalue_rotation) "Undefined" "MultiplyWithRoot" null null))
            (bind _returnvalue_2 (`SceneComponent.K2_GetComponentToWorld` (`/Game/Blueprints/BouncePad.Cube` _returnvalue)))
            (set `self.tp` (`KismetMathLibrary.MakeTransform` (`KismetMathLibrary.MakeVector` (.x (.location _returnvalue_2)) (.y (.location _returnvalue_2)) (+ (.z (.location _returnvalue_2)) 1000.0)) (.rotation _returnvalue_2)))
            (`self.Close Holes`)
            (set `self.RoomAmount` 15)))))
    (else
      (`KismetArrayLibrary.Array_Clear` (`self.OverlappedList`))
      (`self.K2_DestroyActor` (`self.LatestRoom`))
      (`self.Spawn Next Room`))))

(event `Close Holes`
  (for _array_element (`self.exits List`)
    (`|SpawnActorFromClass` "/Game/Blueprints/ProceduralDungeon/WallClose.WallClose_C" (`SceneComponent.K2_GetComponentToWorld` _array_element) "AlwaysSpawn" "MultiplyWithRoot" null null)))

(fn `SpawnMore`
  (`self.Spawn Start Room`)
  (`self.Spawn Next Room`))

(fn `UserConstructionScript`)