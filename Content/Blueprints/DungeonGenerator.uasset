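; Dungeon generator actor that, on BeginPlay, builds a random grid maze and spawns RoomTile actors for it.
; MazeGenerator fills Board with Cells and runs a capped depth-first-style walk, using CheckNeighbors and a Path stack to set door flags.
; GenerateMaze, called from inside that walk on each forward step, spawns a hard-coded 8x8 tile grid spaced by Offset and passes door states to UpdateRoom.
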(event `self.ReceiveBeginPlay`
  (`self.MazeGenerator`))

(fn `CheckNeighbors`
  (params (Cell :type Integer))
  (returns (NeighborsReturn :type "Array of Integer"))
  (locals (Neighbors :type "Array of Integer") (xSize :type Integer))
  (bind _returnvalue (+ Cell 1))
  (bind _returnvalue_2 (- Cell 1))
  (bind _mazesize_x (`KismetMathLibrary.BreakVector` (`self.MazeSize`)))
  (bind _mazesize_x_2 (`KismetMathLibrary.BreakVector` (`self.MazeSize`)))
  (bind _returnvalue_3 (- Cell _mazesize_x_2))
  (bind _returnvalue_4 (+ _mazesize_x Cell))
  (bind _returnvalue_5 (`KismetMathLibrary.FFloor64` _returnvalue_3))
  (bind _returnvalue_6 (`KismetMathLibrary.Conv_Int64ToInt` (`KismetMathLibrary.FFloor64` _returnvalue_4)))
  (set `local.xSize` (`KismetMathLibrary.FTrunc` _mazesize_x_2))
  (if (and (>= _returnvalue_3 0.0) (not (`/Game/Blueprints/Cell.Visited` (`|GetArrayItem` (`self.board`) (`KismetMathLibrary.Conv_Int64ToInt` _returnvalue_5)))))
    (`KismetArrayLibrary.Array_Add` (`local.Neighbors`) (`KismetMathLibrary.Conv_Int64ToInt` _returnvalue_5)))
  (if (and (< _returnvalue_4 (`KismetArrayLibrary.Array_Length` (`self.board`))) (not (`/Game/Blueprints/Cell.Visited` (`|GetArrayItem` (`self.board`) _returnvalue_6))))
    (`KismetArrayLibrary.Array_Add` (`local.Neighbors`) _returnvalue_6))
  (if (and (== (mod _returnvalue (`local.xSize`)) 1) (not (`/Game/Blueprints/Cell.Visited` (`|GetArrayItem` (`self.board`) (`KismetMathLibrary.Conv_Int64ToInt` (`KismetMathLibrary.FFloor64` (`KismetMathLibrary.Conv_IntToDouble` _returnvalue)))))))
    (`KismetArrayLibrary.Array_Add` (`local.Neighbors`) _returnvalue))
  (if (and (!= (mod Cell (`local.xSize`)) 0) (not (`/Game/Blueprints/Cell.Visited` (`|GetArrayItem` (`self.board`) _returnvalue_2))))
    (`KismetArrayLibrary.Array_Add` (`local.Neighbors`) _returnvalue_2))
  (return (`local.Neighbors`)))

(fn `GenerateMaze`
  (locals (lastOne :type "Array of Boolean") (RoomTransform :type "Vector Structure") (xVal :type Integer) (yVal :type Integer) (newRoom :type "/Game/Blueprints/RoomTile Object Reference"))
  (bind (_offset_x _offset_y) (`KismetMathLibrary.BreakVector` (`self.Offset`)))
  (bind (_mazesize_x _mazesize_y) (`KismetMathLibrary.BreakVector` (`self.MazeSize`)))
  (bind _newroom (`local.newRoom`))
  (bind (_mazesize_x_2 _mazesize_y_2) (`KismetMathLibrary.BreakVector` (`self.MazeSize`)))
  (for _index (range 8)
    (set `local.xVal` _index)
    (for _index_2 (range 8)
      (set `local.yVal` _index_2)
      (bind _output_get (set `local.RoomTransform` (`KismetMathLibrary.MakeVector` (* _offset_x (`local.xVal`)) (* _offset_y (`local.yVal`)))))
      (bind _returnvalue (`|SpawnActorFromClass` "/Game/Blueprints/RoomTile.RoomTile_C" (`KismetMathLibrary.Conv_VectorToTransform` _output_get) "Undefined" "MultiplyWithRoot" null null))
      (set `local.newRoom` _returnvalue)
      (if (and (== (`local.xVal`) (- _mazesize_x 1.0)) (== (`local.yVal`) (- _mazesize_y 1.0)))
        (`/Game/Blueprints/RoomTile.UpdateRoom` _newroom (`|MakeArray` false true false false))
        (else
          (`/Game/Blueprints/RoomTile.UpdateRoom` _newroom (`/Game/Blueprints/Cell.status` (`|GetArrayItem` (`self.board`) (`KismetMathLibrary.FTrunc` (+ (* _index _mazesize_y_2) _mazesize_x_2))))))))))

(fn `MazeGenerator`
  (locals (path :type "Array of Integer") (`First Cell` :type "/Game/Blueprints/Cell Object Reference") (whileLoopInt :type Integer) (currentCell :type "/Game/Blueprints/Cell Object Reference") (neighbors :type "Array of Integer") (newCell :type Integer))
  (bind _currentcellindex (`self.currentCellIndex`))
  (bind _path (`local.path`))
  (bind _newcell (`local.newCell`))
  (bind _returnvalue (`KismetArrayLibrary.Array_LastIndex` _path))
  (bind _status (`/Game/Blueprints/Cell.status` (`|GetArrayItem` (`self.board`) _currentcellindex)))
  (for _ (range 50)
    (bind _returnvalue_2 (`|GenericCreateObject` "/Game/Blueprints/Cell.Cell_C"))
    (`KismetArrayLibrary.Array_Add` (`self.board`) _returnvalue_2)
    (bind _output_get (set `self.currentCellIndex` (`self.StartingPos`)))
    (bind _output_get_2 (set `local.First Cell` (`|GetArrayItem` (`self.board`) _output_get)))
    (set `/Game/Blueprints/Cell.status` (`|MakeArray` true false false false) (`local.First Cell`))
    (`KismetArrayLibrary.Array_Set` (`self.board`) 0 _output_get_2)
    (while (< (`local.whileLoopInt`) 10)
      (`/Engine/EditorBlueprintResources/StandardMacros.IncrementInt` (`local.whileLoopInt`)
        (:`  `
          (bind _output_get_3 (set `local.currentCell` (`|GetArrayItem` (`self.board`) (`self.currentCellIndex`))))
          (set `/Game/Blueprints/Cell.Visited` true _output_get_3)
          (bind _neighborsreturn (`self.CheckNeighbors` (`self.currentCellIndex`)))
          (bind _output_get_4 (set `local.neighbors` _neighborsreturn))
          (bind _returnvalue_3 (`KismetArrayLibrary.Array_Length` _output_get_4))
          (if (== _returnvalue_3 0)
            (if (not (== 0 (`KismetArrayLibrary.Array_Length` (`local.path`))))
              (set `self.currentCellIndex` _returnvalue)
              (set `self.currentCellIndex` _returnvalue)
              (`KismetArrayLibrary.Array_Remove` _path _returnvalue))
            (else
              (`KismetArrayLibrary.Array_Add` (`local.path`) (`self.currentCellIndex`))
              (bind _output_get_5 (set `local.newCell` (`KismetMathLibrary.RandomIntegerInRange` 0 _returnvalue_3)))
              (if (> _output_get_5 (`self.currentCellIndex`))
                (if (== (- (`local.newCell`) 1) _currentcellindex)
                  (`KismetArrayLibrary.Array_Set` _status 2 true)
                  (set `self.currentCellIndex` _newcell)
                  (`KismetArrayLibrary.Array_Set` _status 3 true)
                  (else
                    (`KismetArrayLibrary.Array_Set` _status 1 true)
                    (set `self.currentCellIndex` _newcell)
                    (`KismetArrayLibrary.Array_Set` _status 0 true)))
                (elif (== (+ (`local.newCell`) 1) (`self.currentCellIndex`))
                  (`KismetArrayLibrary.Array_Set` _status 3 true)
                  (set `self.currentCellIndex` _newcell)
                  (`KismetArrayLibrary.Array_Set` _status 2 true)
                  (else
                    (`KismetArrayLibrary.Array_Set` _status 0 true)
                    (set `self.currentCellIndex` (`local.newCell`))
                    (`KismetArrayLibrary.Array_Set` _status 1 true))))
              (`self.GenerateMaze`))))))))

(fn `UserConstructionScript`)