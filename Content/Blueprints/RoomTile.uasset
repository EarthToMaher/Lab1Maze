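; Room tile actor with four wall components that can be opened up, likely for assembling connected rooms.
; BeginPlay stores the four walls in an array in a fixed order.
; UpdateRoom takes a boolean status array and destroys the wall component at each index flagged true, leaving openings on those sides.
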(event `self.ReceiveBeginPlay`
  (set `self.Walls` (`|MakeArray` (`self.Wall2`) (`self.Wall3`) (`self.Wall1`) (`self.Wall`))))

(fn `UpdateRoom`
  (params (Status :type "Array of Boolean"))
  (for _index (range (+ (`KismetArrayLibrary.Array_Length` Status) 1))
    (if (`|GetArrayItem` Status _index)
      (`ActorComponent.K2_DestroyComponent` (`|GetArrayItem` (`self.Walls`) _index)))))

(fn `UserConstructionScript`)